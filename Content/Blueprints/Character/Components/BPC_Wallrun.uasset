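; Wallrun component that lets the player character run along and jump off near-vertical walls while falling.
; A looping timer sphere-traces right, then left, using LaunchCharacter to stick to the wall and move along it, with speed and interpolated gravity shaped by player input.
; Starting a run resets the jump and can arrest the fall.
; Jumping launches off the wall normal, and ending a run restores gravity and briefly suppresses re-attachment.
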(event Custom|Initialize
  (params (Character :type Character%20Object%20Reference))
  (bind _output_get (Variables|Default|SetCharacter Character))
  (bind _output_get_2 (Variables|Default|SetCharacter%20Movement (Variables|/Script/Engine.Character|GetCharacterMovement _output_get)))
  (Variables|Default|SetDefault%20Gravity (Variables|/Script/Engine.CharacterMovementComponent|GetGravityScale _output_get_2))
  (Utilities|Time|SetTimerbyEvent (delegate Custom|WallrunUpdateEvent) 0.02 true))

(event Custom|LandEvent
  (CallFunction|WallrunEnd 0.0)
  (Variables|Default|SetWallrunSuppressed false))

(event Custom|JumpEvent
  (CallFunction|WallrunJump))

(event Custom|WallrunUpdateEvent
  (if (not (Variables|Default|GetWallrunSuppressed))
    (CallFunction|WallrunUpdate)))

(event Custom|ResetWallrunSuppression
  (Utilities|Time|ClearTimerbyFunctionName 0 "ResetWallrunSuppression")
  (Variables|Default|SetWallrunSuppressed false))

(event EventTick
  (params (DeltaSeconds :type Float%20%28single-precision%29))
  (if (Variables|Default|GetWallrunning)
    (Utilities|FlowControl|DoOnce false :!label _label
      (:Completed
        (if (Variables|Movement|GetWallrunInitialGravity)
          _
          (else
            (CallFunction|WallrunStopFall)))
        (bind _asbp_player (Utilities|Casting|CastToBP_Player (Variables|Default|GetCharacter)))
        (Default|ResetJump _asbp_player)))
    (else
      (goto _label Reset))))

(fn WallrunUpdate
  (bind _character_movement (Variables|Default|GetCharacter%20Movement))
  (bind _onwall (CallFunction|WallrunMovement (Transformation|GetActorLocation (Variables|Default|GetCharacter)) (.Right (Utilities|WallrunEndVectors)) 2e+01 -1.0))
  (if _onwall
    (bind _output_get (Variables|Default|SetWallrunning true))
    (Variables|Default|SetWallrunningR _output_get)
    (Variables|Default|SetWallrunningL false)
    (Variables|/Script/Engine.CharacterMovementComponent|SetGravityScale _character_movement (Math|Interpolation|FInterpTo (Variables|/Script/Engine.CharacterMovementComponent|GetGravityScale _character_movement) (Utilities|WallrunGetGravity) (Utilities|Time|GetWorldDeltaSeconds) 1e+01) :!label _label)
    (elif (Variables|Default|GetWallrunningR)
      (CallFunction|WallrunEnd 1.0)
      (else
        (bind _onwall_2 (CallFunction|WallrunMovement (Transformation|GetActorLocation (Variables|Default|GetCharacter)) (.Left (Utilities|WallrunEndVectors)) 2e+01 1.0))
        (if _onwall_2
          (Variables|Default|SetWallrunning true)
          (Variables|Default|SetWallrunningR false)
          (Variables|Default|SetWallrunningL true)
          (goto _label)
          (else
            (CallFunction|WallrunEnd 1.0)))))))

(fn WallrunMovement
  (params (Start :type Vector) (End :type Vector) (Radius :type Float%20%28single-precision%29) (Direction :type Float%20%28single-precision%29))
  (bind _outhit (Collision|SphereTraceByChannel Start End Radius "TraceTypeQuery1" false 0 (select (Variables|Default|GetDEBUG) "Persistent" "None")))
  (if (and (.bblockinghit _outhit) (AI|Components|NavMovement|IsFalling (Variables|Default|GetCharacter%20Movement)))
    (if (.ReturnValue (Utilities|ValidWallrunVector (.normal _outhit) -0.52 0.52))
      (Variables|Default|SetWallrunNormal (.OutVec (Utilities|ValidWallrunVector (.normal _outhit) -0.52 0.52)))
      ;[1 1 1] stick to wall
      (Character|LaunchCharacter (Variables|Default|GetCharacter) (Utilities|PlayertoWallVector) false false)
      ;[1 1 1] move forward
      (Character|LaunchCharacter (Variables|Default|GetCharacter) (Utilities|WallrunSpeed Direction) true (not (Variables|Movement|GetWallrunGravity)))
      (return true)
      (else
        _)))
  (return false))

(fn WallrunEnd
  (params (ResetTime :type Float%20%28single-precision%29))
  (if (Variables|Default|GetWallrunning)
    (Variables|Default|SetWallrunning false)
    (Variables|Default|SetWallrunningR false)
    (Variables|Default|SetWallrunningL false)
    (Variables|/Script/Engine.CharacterMovementComponent|SetGravityScale (Variables|Default|GetCharacter%20Movement) (Variables|Default|GetDefault%20Gravity))
    (CallFunction|SuppressWallrun ResetTime)))

(fn SuppressWallrun
  (params (Delay :type Float%20%28single-precision%29))
  (Variables|Default|SetWallrunSuppressed true)
  (Utilities|Time|SetTimerbyFunctionName 0 "ResetWallrunSuppression" Delay))

(fn WallrunJump
  (bind _wallrunnormal (Variables|Default|GetWallrunNormal))
  (bind _wallrunjumpforce (Variables|Movement|GetWallrunJumpForce))
  (if (Variables|Default|GetWallrunning)
    (CallFunction|WallrunEnd 0.25)
    (Character|LaunchCharacter (Variables|Default|GetCharacter) (Math|Vector|MakeVector (* (.x _wallrunnormal) _wallrunjumpforce) (* (.y _wallrunnormal) _wallrunjumpforce) (Variables|Movement|GetWallrunJumpHeight)) false true)))

(fn WallrunStopFall
  (bind _character_movement (Variables|Default|GetCharacter%20Movement))
  (bind _returnvalue (Pawn|Components|CharacterMovement|GetLastUpdateVelocity _character_movement))
  (Variables|/Script/Engine.MovementComponent|SetVelocity _character_movement (Math|Vector|MakeVector (.x _returnvalue) (.y _returnvalue) 1.5e+02))
  (return))