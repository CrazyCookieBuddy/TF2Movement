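; Player component that manages a pair of linked portals, fired from the character's camera and stored in a map by key.
; ShootPortal line-traces along the camera forward and spawns a BP_Portal aligned to the hit normal, replacing that key's existing portal only on a blocking hit.
; When the opposite portal exists, both exchange render targets through SetRT.
; Helper functions destroy portals by key or by reference.
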(event EventInitialize
  (params (Player :type Character%20Object%20Reference))
  (bind _asbp_player (Utilities|Casting|CastToBP_Player Player))
  (Variables|Default|SetCharacter _asbp_player))

(fn ShootPortal
  (params (Portal :type Integer))
  (bind _returnvalue (Class|KismetSystemLibrary|MakeLiteralInteger 1))
  (bind _returnvalue_2 (Class|KismetSystemLibrary|MakeLiteralInteger))
  (bind _character (Variables|Default|GetCharacter))
  (bind _portals (Variables|Default|GetPortals))
  (bind _character_2 (Variables|Default|GetCharacter))
  (bind _returnvalue_3 (Utilities|Select :Index Portal :Option%200 _returnvalue :Option%201 _returnvalue_2))
  (bind _camera (Variables|/Game/Blueprints/Character/BP_Player.BP_Player_C|GetCamera _character))
  (bind _camera_2 (Variables|/Game/Blueprints/Character/BP_Player.BP_Player_C|GetCamera _character_2))
  (bind _returnvalue_4 (Transformation|GetWorldLocation _camera_2))
  (bind (_value _returnvalue_5) (Utilities|Map|Find _portals _returnvalue_3))
  (bind _returnvalue_6 (Transformation|GetWorldLocation _camera))
  (if (.ReturnValue (Utilities|Map|Find (Variables|Default|GetPortals) Portal))
    (bind _outhit (Collision|LineTraceByChannel _returnvalue_6 (+ _returnvalue_6 (* (Math|Vector|GetForwardVector _camera) 1e+04)) "TraceTypeQuery1" false 0 "None"))
    (if (.bblockinghit _outhit)
      (CallFunction|DestroyPortalwithKey Portal)
      (bind _outhit_2 (Collision|LineTraceByChannel _returnvalue_4 (+ _returnvalue_4 (* (Math|Vector|GetForwardVector _camera_2) 1e+04)) "TraceTypeQuery1" false 0 "None" :!label _label))
      (bind _returnvalue_7 (Game|SpawnActorfromClass "/Game/Blueprints/Portals/BP_Portal.BP_Portal_C" (Math|Transform|MakeTransform (.location _outhit_2) (Math|Rotator|MakeRotfromZ (.normal _outhit_2))) "Undefined" 0 (Game|Player|GetPlayerPawn 0)))
      (Utilities|Map|Add _portals Portal _returnvalue_7)
      (if _returnvalue_5
        (Default|SetRT _returnvalue_7 (Variables|/Game/Blueprints/Portals/BP_Portal.BP_Portal_C|GetRT _value))
        (Default|SetRT _value (Variables|/Game/Blueprints/Portals/BP_Portal.BP_Portal_C|GetRT _returnvalue_7))))
    (else
      (goto _label))))

(fn DestroyPortalwithKey
  (params (Key :type Integer%20%28by%20ref%29))
  (bind _portals (Variables|Default|GetPortals))
  (bind (_value _returnvalue) (Utilities|Map|Find _portals Key))
  (if _returnvalue
    (Actor|DestroyActor _value))
  (Utilities|Map|Remove _portals Key))

(fn DestroyPortal
  (params (Portal :type BP%20Portal%20Object%20Reference))
  (bind _values (Utilities|Map|Values (Variables|Default|GetPortals)))
  (if (not (== (Utilities|Array|FindItem _values Portal) -1))
    (Utilities|Map|Remove (Variables|Default|GetPortals) (Utilities|Array|FindItem _values Portal))
    (Actor|DestroyActor Portal)))