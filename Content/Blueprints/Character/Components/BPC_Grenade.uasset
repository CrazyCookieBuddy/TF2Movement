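; Grenade component for BP_Player that previews the throw arc with one bounce while a grenade is held; Throw is an empty stub.
; Each Tick, Predict traces a colliding projectile path from above the character along camera forward, drawn as debug.
; It then draws a non-colliding bounce arc from the hit, mirroring the incoming velocity and scaling it by impact speed.
; BeginPlay also starts a looping PredictLoop timer, whose event is empty.
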(event Custom|PredictLoop)

(event EventInitialize
  (params (Player :type Character%20Object%20Reference))
  (bind _asbp_player (Utilities|Casting|CastToBP_Player Player))
  (Variables|Default|SetCharacter _asbp_player))

(event EventBeginPlay
  (bind _returnvalue (Utilities|Time|SetTimerbyEvent (delegate Custom|PredictLoop) 0.2 true))
  (Variables|Default|SetPredictLoopTimer _returnvalue))

(event EventTick
  (params (DeltaSeconds :type Float%20%28single-precision%29))
  (if (Variables|/Game/Blueprints/Character/BP_Player.BP_Player_C|GetHoldingGrenade (Variables|Default|GetCharacter))
    (CallFunction|Predict)))

(fn Predict
  (bind _character (Variables|Default|GetCharacter))
  (bind _returnvalue (Transformation|GetActorLocation _character))
  (bind (_x _y _z) (Math|Vector|BreakVector _returnvalue))
  (bind _predictresult (Class|GameplayStatics|BlueprintPredictProjectilePathAdvanced (Utilities|Struct|MakePredictProjectilePathParams (Math|Vector|MakeVector _x _y (+ _z (Variables|Default|GetThrowOffset))) (* (Math|Vector|GetForwardVector (Variables|/Game/Blueprints/Character/BP_Player.BP_Player_C|GetCamera _character)) (Variables|Default|GetThrowForce)) true 4.0 5.0 true "ECC_WorldStatic" "ObjectTypeQuery1" (Utilities|Array|MakeArray _character) 2e+01 0.0 "ForOneFrame" 0.2)))
  (Variables|Default|SetPath%20Data (.PathData (Utilities|Struct|BreakPredictProjectilePathResult _predictresult)))
  (Class|GameplayStatics|BlueprintPredictProjectilePathAdvanced (Utilities|Struct|MakePredictProjectilePathParams (.Location (Collision|BreakHitResult (.HitResult (Utilities|Struct|BreakPredictProjectilePathResult _predictresult)))) (* (Math|Vector|MirrorVectorbyNormal (.Velocity (Utilities|Struct|BreakPredictProjectilePathPointData (Utilities|Array|Get(acopy) (Variables|Default|GetPath%20Data) (- (Utilities|Array|Length (Variables|Default|GetPath%20Data)) 2)))) (Math|Vector|Normalize (* (Math|Vector|ProjectVectorontoPlane (- (.Location (Collision|BreakHitResult (.HitResult (Utilities|Struct|BreakPredictProjectilePathResult _predictresult)))) (.Location (Utilities|Struct|BreakPredictProjectilePathPointData (Utilities|Array|Get(acopy) (Variables|Default|GetPath%20Data) (- (Utilities|Array|Length (Variables|Default|GetPath%20Data)) 2))))) (.ImpactNormal (Collision|BreakHitResult (.HitResult (Utilities|Struct|BreakPredictProjectilePathResult _predictresult))))) -1.0))) (* (Math|Float|MapRangeClamped (Math|Vector|VectorLength (.Velocity (Utilities|Struct|BreakPredictProjectilePathPointData (Utilities|Array|Get(acopy) (Variables|Default|GetPath%20Data) (- (Utilities|Array|Length (Variables|Default|GetPath%20Data)) 1))))) 1.5e+03 2.2e+03 0.0 1.0) -1.0)) false 0.0 5.0 true "ECC_WorldStatic" "ObjectTypeQuery1" 0 2e+01 0.0 "ForOneFrame" 0.2)))

(fn Throw)