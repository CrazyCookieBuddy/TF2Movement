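; Player shooting component that fires the current gun with sound, impact and optional trail effects, and recoil.
; A looping timer at the gun's shot delay drives a gate opened and closed by trigger events, closing after each semi-auto shot.
; Each shot traces from camera to find the aim point, then from muzzle toward it, without applying damage.
; Recoil adds random yaw and fixed upward pitch, with a crouch modifier.
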(event Custom|Initialize
  (params (Character :type Character%20Object%20Reference))
  (bind _asbp_player (Utilities|Casting|CastToBP_Player Character))
  (bind _output_get (Variables|Default|SetCharacter _asbp_player))
  (bind _output_get_2 (Variables|Default|SetGun (Variables|/Game/Blueprints/Character/BP_Player.BP_Player_C|GetGun _output_get)))
  (Development|PrintString (Utilities|String|Append "Gun: " (Utilities|String|ToString(Name) (.Name (Utilities|Struct|BreakS_Gun _output_get_2))) "              " "Sound:" (Utilities|GetDisplayName (.Sound (Utilities|Struct|BreakS_Gun _output_get_2))))))

(event Custom|UpdateGun
  (params (Gun :type S%20Gun%20Structure))
  (Variables|Default|SetGun Gun))

(event Custom|ShootGateOpen
  (bind _gun (Variables|Default|GetGun))
  (if (not (Utilities|Time|IsValidTimerHandle (Variables|Default|GetAttemtpShootHandler)))
    (bind _returnvalue (Utilities|Time|SetTimerbyEvent (delegate Custom|AttemptShoot) (.shotdelay _gun) true (* (.shotdelay _gun) -1.0) :!label _label))
    (Variables|Default|SetAttemtpShootHandler _returnvalue)
    (Utilities|FlowControl|Gate false) ; enters at Open
    (elif (not (Variables|Default|GetShooting))
      (goto _label)
      (else
        (Utilities|FlowControl|Gate false) ; enters at Open
      ))))

(event Custom|ShootGateClose
  (Utilities|FlowControl|Gate false) ; enters at Close
)

(event Custom|Recoil
  (bind _gun (Variables|Default|GetGun))
  (bind _character (Variables|Default|GetCharacter))
  (bind (_x _y _z) (Math|Vector|BreakVector (.recoil _gun)))
  (Pawn|Input|AddControllerYawInput _character (Math|Random|RandomFloatinRange (* _x -1.0) _x)) ; Horizontal
  (Pawn|Input|AddControllerPitchInput _character (* _z -1.0)) ; Vertical
)

(event Custom|AttemptShoot
  (Variables|Default|SetShooting false)
  (Utilities|FlowControl|Gate false
    (:Exit
      (CallFunction|Shoot)
      (Variables|Default|SetShooting true)
      (if (not (.isauto (Variables|Default|GetGun)))
        (CallFunction|ShootGateClose)))))

(fn Shoot
  (CallFunction|LinetraceShot)
  (Audio|PlaySoundatLocation (.Sound (Utilities|Struct|BreakS_Gun (Variables|Default|GetGun))) (Transformation|GetWorldLocation (Variables|/Game/Blueprints/Character/BP_Player.BP_Player_C|GetShotLocation (Variables|Default|GetCharacter))) "0, 0, 0" 1.0 1.0 0.0 0 0 0)
  (CallFunction|StartRecoil))

(fn StartRecoil
  (bind _gun (Variables|Default|GetGun))
  (bind _character (Variables|Default|GetCharacter))
  (bind (_x _y _z) (Math|Vector|BreakVector (.recoil _gun)))
  (bind _returnvalue (* _z -1.0))
  (Pawn|Input|AddControllerYawInput _character (* (Math|Random|RandomFloatinRange (* _x -1.0) _x) (Variables|Default|GetCrouchModifier))) ; Horizontal
  (Pawn|Input|AddControllerPitchInput _character (Math|Float|SelectFloat _returnvalue (* _returnvalue (Variables|Default|GetCrouchModifier)) (not (Variables|/Script/Engine.Character|GetbIsCrouched (Variables|Default|GetCharacter))))) ; Vertical
)

(fn LinetraceShot
  (bind _character (Variables|Default|GetCharacter))
  (bind _character_2 (Variables|Default|GetCharacter))
  (bind _character_3 (Variables|Default|GetCharacter))
  (bind _camera (Variables|/Game/Blueprints/Character/BP_Player.BP_Player_C|GetCamera _character))
  (bind _camera_2 (Variables|/Game/Blueprints/Character/BP_Player.BP_Player_C|GetCamera _character_2))
  (bind _camera_3 (Variables|/Game/Blueprints/Character/BP_Player.BP_Player_C|GetCamera _character_3))
  (bind _returnvalue (Transformation|GetWorldLocation _camera))
  (bind _returnvalue_2 (Math|Vector|GetForwardVector _camera))
  (bind _returnvalue_3 (Transformation|GetWorldLocation _camera_2))
  (bind _returnvalue_4 (* _returnvalue_2 1e+04))
  (bind _returnvalue_5 (+ _returnvalue _returnvalue_4))
  (Variables|Default|SetShotQueued false)
  (bind _outhit (Collision|LineTraceByChannel _returnvalue_3 (+ _returnvalue_3 (* (Math|Vector|GetForwardVector _camera_2) 1e+04)) "TraceTypeQuery2" true 0 "None" true "(R=1.000000,G=0.000000,B=0.000000,A=1.000000)" "(R=0.000000,G=1.000000,B=0.000000,A=1.000000)" 1.0))
  (bind _outhit_2 (Collision|LineTraceByChannel (Transformation|GetWorldLocation (Variables|/Game/Blueprints/Character/BP_Player.BP_Player_C|GetShotLocation (Variables|Default|GetCharacter))) (Math|Vector|SelectVector (+ (.location _outhit) (* (Math|Vector|GetUnitDirection(Vector) _returnvalue_5 (.location _outhit)) -1e+01)) _returnvalue_5 (.bblockinghit _outhit)) "TraceTypeQuery2" true 0 "None" true "(R=1.000000,G=0.000000,B=0.000000,A=1.000000)" "(R=0.000000,G=1.000000,B=0.000000,A=1.000000)" 1.0))
  (if (.bblockinghit _outhit_2)
    (Niagara|SpawnSystematLocation "/Game/Art/VFX/Bullets/FX_Impact_System.FX_Impact_System" (.location _outhit_2) (Math|Conversions|RotationFromXVector (.impactnormal _outhit_2)) "1.000000,1.000000,1.000000" true true "AutoRelease" false)
    (LocalVariables|SetBeamEnd (.location _outhit_2))
    (else
      (LocalVariables|SetBeamEnd (+ (Transformation|GetWorldLocation _camera_3) (* (Math|Vector|GetForwardVector _camera_3) 1e+04)))))
  (if (LocalVariables|GetShootTrail)
    (bind _returnvalue_6 (Niagara|SpawnSystematLocation "/Game/Art/VFX/Bullets/FX_Shot_System.FX_Shot_System" (Transformation|GetWorldLocation (Variables|/Game/Blueprints/Character/BP_Player.BP_Player_C|GetShotLocation (Variables|Default|GetCharacter)))))
    (Effects|Components|ParticleSystem|SetVectorParameter _returnvalue_6 "EndPoint" (LocalVariables|GetBeamEnd)))
  (return (.hitactor _outhit_2)))