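; Character component that handles crouch toggling and momentum slides for the player.
; A crouch press on the ground starts a slide if allowed or toggles crouch, while an airborne press toggles a queued slide.
; Slides plane-constrain movement, cut friction and add a floor-aligned impulse on flat or downhill ground.
; A looping timer behind a gate ends slides at low speed and restores cached movement defaults.
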(event Custom|CheckQueue
  (if (Variables|Default|GetSlideQueued)
    (if (> (Variables|Default|GetSlideRetry) 3)
      (Variables|Default|SetSlideRetry 0)
      (Variables|Default|SetSlideQueued false)
      (else
        (Math|Integer|IncrementInt (Variables|Default|GetSlideRetry)
          (:%20%20
            (CallFunction|SlideStart)))))))

(event Custom|SlideUpdateEvent
  (Utilities|FlowControl|Gate true
    (:Exit
      (CallFunction|SlideUpdate))))

(event Custom|CrouchSlideEvent
  (if (Pawn|Components|CharacterMovement|IsWalking (Variables|Default|GetCharacter%20Movement))
    (if (Utilities|CanSlide)
      (CallFunction|SlideStart)
      (elif (AI|Components|NavMovement|IsCrouching (Variables|Default|GetCharacter%20Movement))
        (CallFunction|CrouchEnd)
        (else
          (CallFunction|CrouchStart))))
    (else
      (Variables|Default|SetSlideQueued (not (Variables|Default|GetSlideQueued))))))

(event Custom|CloseSlideGate
  (Utilities|FlowControl|Gate true) ; enters at Close
)

(event Custom|OpenSlideGate
  (Utilities|FlowControl|Gate true) ; enters at Open
)

(event EventInitialize
  (params (Player :type Character%20Object%20Reference))
  ;[1 1 1] init
  (bind _output_get (Variables|Default|SetCharacter Player))
  (Variables|Default|SetCharacter%20Movement (Variables|/Script/Engine.Character|GetCharacterMovement _output_get))
  (Variables|Default|SetDefaultGroundFriction (Variables|/Script/Engine.CharacterMovementComponent|GetGroundFriction (Variables|/Script/Engine.Character|GetCharacterMovement _output_get)))
  (Variables|Default|SetDefaultBrakingDecel (Variables|/Script/Engine.CharacterMovementComponent|GetBrakingDecelerationWalking (Variables|/Script/Engine.Character|GetCharacterMovement _output_get)))
  (Variables|Default|SetDefaultMaxWalkCrouched (Variables|/Script/Engine.CharacterMovementComponent|GetMaxWalkSpeedCrouched (Variables|/Script/Engine.Character|GetCharacterMovement _output_get)))
  (Variables|Default|SetDefaultMaxWalk (Variables|/Script/Engine.CharacterMovementComponent|GetMaxWalkSpeed (Variables|/Script/Engine.Character|GetCharacterMovement _output_get)))
  (Utilities|Time|SetTimerbyEvent (delegate Custom|SlideUpdateEvent) 0.02 true))

(fn SlideStart
  (bind _character_movement (Variables|Default|GetCharacter%20Movement))
  (bind _character_movement_2 (Variables|Default|GetCharacter%20Movement))
  (bind _character_movement_3 (Variables|Default|GetCharacter%20Movement))
  (if (and (Utilities|CanSlide) (Pawn|Components|CharacterMovement|IsWalking (Variables|Default|GetCharacter%20Movement)))
    (Character|Crouch (Variables|Default|GetCharacter))
    (Class|MovementComponent|SetPlaneConstraintfromVectors _character_movement_2 (Math|Vector|Normalize (Variables|/Script/Engine.MovementComponent|GetVelocity (Variables|Default|GetCharacter%20Movement))) (Transformation|GetActorUpVector (Variables|Default|GetCharacter)))
    (Class|MovementComponent|SetPlaneConstraintEnabled _character_movement_2 true)
    (bind _slidevector (Utilities|GetSlideVector))
    (if (<= (.Z (Math|Vector|BreakVector _slidevector)) 0.02)
      (Physics|AddImpulse (Variables|Default|GetCharacter%20Movement) (* _slidevector (Variables|Default|GetSlideImpulse)) true)
      (Variables|/Script/Engine.CharacterMovementComponent|SetGroundFriction _character_movement 0.0)
      (Variables|/Script/Engine.CharacterMovementComponent|SetBrakingDecelerationWalking _character_movement 5e+02)
      (Variables|/Script/Engine.CharacterMovementComponent|SetMaxWalkSpeedCrouched _character_movement 0.0)
      (else
        (Variables|/Script/Engine.CharacterMovementComponent|SetGroundFriction _character_movement_3 0.0)
        (Variables|/Script/Engine.CharacterMovementComponent|SetBrakingDecelerationWalking _character_movement_3 8e+02)
        (Variables|/Script/Engine.CharacterMovementComponent|SetMaxWalkSpeedCrouched _character_movement_3 0.0)))
    (Variables|Default|SetSlideQueued false)
    (Variables|Default|SetSliding true)
    (CallFunction|OpenSlideGate)
    (elif (Variables|Default|GetSlideQueued)
      (Utilities|Time|SetTimerbyFunctionName 0 "CheckQueue" 0.2))))

(fn SlideEnd
  (params (Crouch :type Boolean))
  (if (Variables|Default|GetSliding)
    (Class|MovementComponent|SetPlaneConstraintEnabled (Variables|Default|GetCharacter%20Movement) false)
    (CallFunction|ResetDefault)
    (Variables|Default|SetSliding false)
    (CallFunction|CloseSlideGate)
    (Character|UnCrouch (Variables|Default|GetCharacter))))

(fn CrouchStart
  (Character|Crouch (Variables|Default|GetCharacter)))

(fn CrouchEnd
  (Character|UnCrouch (Variables|Default|GetCharacter))
  (CallFunction|ResetDefault))

(fn SlideUpdate
  (if (Variables|Default|GetSliding)
    (if (<= (Math|Vector|VectorLength (Variables|/Script/Engine.MovementComponent|GetVelocity (Variables|Default|GetCharacter%20Movement))) 3e+02)
      (CallFunction|SlideEnd true))))

(fn ResetDefault
  (bind _character_movement (Variables|Default|GetCharacter%20Movement))
  (Variables|/Script/Engine.CharacterMovementComponent|SetGroundFriction _character_movement (Variables|Default|GetDefaultGroundFriction))
  (Variables|/Script/Engine.CharacterMovementComponent|SetBrakingDecelerationWalking _character_movement (Variables|Default|GetDefaultBrakingDecel))
  (Variables|/Script/Engine.CharacterMovementComponent|SetMaxWalkSpeedCrouched _character_movement (Variables|Default|GetDefaultMaxWalkCrouched))
  (Variables|/Script/Engine.CharacterMovementComponent|SetMaxWalkSpeed _character_movement (Variables|Default|GetDefaultMaxWalk)))