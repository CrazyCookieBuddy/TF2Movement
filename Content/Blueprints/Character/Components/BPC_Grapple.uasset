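; Player grapple component that fires a visible cable at a traced target and pulls the character to it.
; A sphere trace sets the goal and cooldown (shorter on a miss), Tick extends the spawned CableActor, and a distance-based delay precedes launch.
; A fast looping timer lerps the character with sweep until close or timed out, queuing a step-up on arrival.
; A second timer feeds cooldown progress to the abilities widget.
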(event Custom|TryMovePlayer
  (params (Delay :type Float%20%28single-precision%29) (Goal :type Vector))
  (bind _character (Variables|Default|GetCharacter))
  (Variables|Default|SetGoal Goal)
  (Utilities|FlowControl|Delay Delay)
  (Character|LaunchCharacter (Variables|Default|GetCharacter) "0, 0,200.000000" false false)
  (Variables|Default|SetStartPosition (Transformation|GetActorLocation (Variables|Default|GetCharacter)))
  (Character|LaunchCharacter _character (* (Transformation|GetVelocity _character) -0.5) false false)
  (Utilities|Time|SetTimerbyEvent (delegate Custom|Launch) 0.005 true))

(event Custom|TryGrapple
  (if (and (Utilities|CheckCooldown) (Variables|Default|GetCanGrapple))
    (CallFunction|ShootGrapple)))

(event Custom|CooldownTimer
  (bind _cooldown (Variables|Default|GetCooldown))
  (if (Variables|Default|GetCanGrapple)
    (if (< (Variables|Default|GetCooldownTime) _cooldown)
      (Variables|Default|SetCooldownTime (+ (Variables|Default|GetCooldownTime) 0.1))
      ;[1 1 1] set UI
      (Default|SetPercentage (Variables|/Game/Blueprints/UI/WBP_Abilities.WBP_Abilities_C|GetM_WBP_Ability (Variables|/Game/Blueprints/Character/BP_Player.BP_Player_C|GetAbilitiesWidget (Variables|Default|GetCharacter))) (Math|Float|MapRangeClamped (Variables|Default|GetCooldownTime) 0.0 _cooldown 0.0 1.0)))))

(event Custom|TryStepupPlayer
  (bind (_returnvalue _point1 _point2) (CallFunction|CheckStepupSpace))
  (if _returnvalue
    (Default|StepUp (Variables|Default|GetCharacter) (Utilities|Array|MakeArray _point1 _point2))))

(event Custom|Launch
  (CallFunction|GrappleLaunch))

(event Custom|StopGrapple
  (Variables|Default|SetCanGrapple true)
  (Variables|Default|SetUpdateCableBool false)
  (Utilities|Time|ClearTimerbyFunctionName 0 "Launch")
  (Variables|Default|SetLaunchCounter 0)
  (Rendering|SetActorHiddenInGame (Variables|Components|GetGrapplingCable) true)
  (if (Variables|Default|GetQueueStepup)
    (Variables|Default|SetQueueStepup false)
    (CallFunction|TryStepupPlayer)))

(event EventTick
  (params (DeltaSeconds :type Float%20%28single-precision%29))
  (if (Variables|Default|GetUpdateCableBool)
    (Utilities|UpdateCable (Math|Vector|Lerp(Vector) (Transformation|GetActorLocation (Variables|Components|GetGrapplingCable)) (Variables|Default|GetGoal) (Variables|Default|GetUpdateCableAlpha)))
    (Variables|Default|SetUpdateCableAlpha (+ (Variables|Default|GetUpdateCableAlpha) 0.01))
    (else
      (Variables|Default|SetUpdateCableAlpha 0.0))))

(event EventInitialize
  (params (Player :type Character%20Object%20Reference))
  (bind _asbp_player (Utilities|Casting|CastToBP_Player Player))
  (Variables|Default|SetCharacter _asbp_player)
  (bind _returnvalue (Game|SpawnActorfromClass "/Script/CableComponent.CableActor" (Math|Transform|MakeTransform "0, 0, 0") "Undefined" 0 0))
  (bind _output_get (Variables|Components|SetGrapplingCable _returnvalue))
  (Variables|/Script/CableComponent.CableComponent|SetbEnableStiffness (Variables|/Script/CableComponent.CableActor|GetCableComponent _output_get) true)
  (Rendering|SetActorHiddenInGame _output_get true)
  (Utilities|Time|SetTimerbyEvent (delegate Custom|CooldownTimer) 0.1 true))

(fn ShootGrapple
  (bind (_outhit _returnvalue) (CallFunction|TracefromtoCenter (Transformation|GetWorldLocation (Variables|/Game/Blueprints/Character/BP_Player.BP_Player_C|GetShotLocation (Variables|Default|GetCharacter))) (Variables|Default|GetGrappleLength) false 15.0 "None"))
  (Variables|Default|SetHitImpact _outhit)
  (Variables|Default|SetCooldownTime 0.0)
  (if _returnvalue
    (Variables|Default|SetCooldown 4.0)
    (bind _cabletime (CallFunction|MoveCable (Math|Vector|SelectVector (.TraceEnd (Collision|BreakHitResult _outhit)) (.ImpactPoint (Collision|BreakHitResult _outhit)) (.bBlockingHit (Collision|BreakHitResult _outhit)))))
    (CallFunction|TryMovePlayer _cabletime (Math|Vector|SelectVector (.TraceEnd (Collision|BreakHitResult _outhit)) (.ImpactPoint (Collision|BreakHitResult _outhit)) (.bBlockingHit (Collision|BreakHitResult _outhit))))
    (else
      (Variables|Default|SetCooldown 0.5))))

(fn MoveCable
  (params (Goal :type Vector))
  (Rendering|SetActorHiddenInGame (Variables|Components|GetGrapplingCable) false)
  (Variables|Default|SetUpdateCableBool true)
  (return (/ (Math|Vector|Distance(Vector) Goal (Transformation|GetActorLocation (Variables|Default|GetCharacter))) 4.5e+03)))

(fn GrappleLaunch
  (if true
    (Transformation|SetActorLocation (Variables|Default|GetCharacter) (Math|Vector|Lerp(Vector) (Variables|Default|GetStartPosition) (Variables|Default|GetGoal) (* (Variables|Default|GetLaunchCounter) 0.01)) true false)
    (else
      (Character|LaunchCharacter (Variables|Default|GetCharacter) (* (Utilities|GetGrappleDirection (Variables|Default|GetGoal)) (Variables|Default|GetStrength)) false false)))
  (Math|Integer|IncrementInt (Variables|Default|GetLaunchCounter)
    (:%20%20
      (if (or (> (Variables|Default|GetLaunchCounter) 200) (< (Math|Vector|Distance(Vector) (Variables|Default|GetGoal) (Transformation|GetActorLocation (Variables|Default|GetCharacter))) (Variables|Default|GetMaxDistance)))
        (CallFunction|StopGrapple)
        (if (< (Math|Vector|Distance(Vector) (Variables|Default|GetGoal) (Transformation|GetActorLocation (Variables|Default|GetCharacter))) (Variables|Default|GetMaxDistance))
          (Variables|Default|SetQueueStepup true))))))