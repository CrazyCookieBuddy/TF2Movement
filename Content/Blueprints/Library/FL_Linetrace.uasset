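; Blueprint function library of trace helpers for camera-centered targeting and step-up clearance checks.
; TraceFromToCenter traces from the BP_Player camera, then line or sphere traces from a second start point to just past that hit, or to full range on a miss.
; CheckStepupSpace sphere-traces up along a hit surface and box-traces back against its normal, returning whether both are clear plus two path points, with persistent debug drawing.
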(fn TracefromtoCenter
  (params (SecondStartPoint :type Vector) (Length :type Float%20%28single-precision%29) (Linetrace :type Boolean) (SpheretraceRadius :type Float%20%28single-precision%29) (DrawDebugType :type EDrawDebugTrace%20Enum :default "None"))
  (bind _returnvalue (Game|Player|GetPlayerPawn 0))
  (bind _returnvalue_2 (Game|Player|GetPlayerPawn 0))
  (bind _asbp_player (Utilities|Casting|CastToBP_Player _returnvalue))
  (bind _asbp_player_2 (Utilities|Casting|CastToBP_Player _returnvalue_2))
  (bind _camera (Variables|/Game/Blueprints/Character/BP_Player.BP_Player_C|GetCamera _asbp_player))
  (bind _camera_2 (Variables|/Game/Blueprints/Character/BP_Player.BP_Player_C|GetCamera _asbp_player_2))
  (bind _returnvalue_3 (Transformation|GetWorldLocation _camera))
  (bind _returnvalue_4 (Math|Vector|GetForwardVector _camera))
  (bind _returnvalue_5 (Transformation|GetWorldLocation _camera_2))
  (bind _returnvalue_6 (* _returnvalue_4 Length))
  (bind _returnvalue_7 (+ _returnvalue_3 _returnvalue_6))
  (bind _outhit (Collision|LineTraceByChannel 0 _returnvalue_5 (+ _returnvalue_5 (* (Math|Vector|GetForwardVector _camera_2) Length)) "TraceTypeQuery2" true 0 "None" true "(R=1.000000,G=0.000000,B=0.000000,A=1.000000)" "(R=0.000000,G=1.000000,B=0.000000,A=1.000000)" 1.0))
  (if Linetrace
    (bind (_outhit_2 _returnvalue_8) (Collision|LineTraceByChannel 0 SecondStartPoint (Math|Vector|SelectVector (+ (.location _outhit) (* (Math|Vector|GetUnitDirection(Vector) _returnvalue_7 (.location _outhit)) -1e+01)) _returnvalue_7 (.bblockinghit _outhit)) "TraceTypeQuery1" false 0 DrawDebugType))
    (return _outhit_2 _returnvalue_8)
    (else
      (bind (_outhit_3 _returnvalue_9) (Collision|SphereTraceByChannel 0 SecondStartPoint (Math|Vector|SelectVector (+ (.location _outhit) (* (Math|Vector|GetUnitDirection(Vector) _returnvalue_7 (.location _outhit)) -1e+01)) _returnvalue_7 (.bblockinghit _outhit)) SpheretraceRadius "TraceTypeQuery1" false 0 DrawDebugType))
      (return _outhit_3 _returnvalue_9))))

(fn CheckStepupSpace
  (params (Hit :type Hit%20Result%20Structure) (Away :type Float%20%28single-precision%29) (Up :type Float%20%28single-precision%29) (Back :type Float%20%28single-precision%29) (BoxSize :type Vector :default "55.000000,55.000000,96.000000") (SphereRadius :type Float%20%28single-precision%29))
  (bind _returnvalue (Math|Vector|VectorUp))
  (bind _returnvalue_2 (* (.impactnormal Hit) Back))
  (bind _returnvalue_3 (* (.impactnormal Hit) Away))
  (bind _returnvalue_4 (Math|Vector|ProjectVectorontoPlane _returnvalue (.impactnormal Hit)))
  (bind _returnvalue_5 (+ (.location Hit) _returnvalue_3))
  (bind _returnvalue_6 (Math|Vector|Normalize _returnvalue_4))
  (bind _returnvalue_7 (* _returnvalue_6 Up))
  (bind _returnvalue_8 (+ _returnvalue_5 _returnvalue_7))
  (bind _returnvalue_9 (- _returnvalue_8 _returnvalue_2))
  ;[1 1 1] along plane
  (bind _returnvalue_10 (Collision|SphereTraceByChannel 0 _returnvalue_5 _returnvalue_8 SphereRadius "TraceTypeQuery1" false 0 "Persistent"))
  (bind _returnvalue_11 (Collision|BoxTraceByChannel 0 _returnvalue_8 _returnvalue_9 BoxSize (Math|Rotator|FindLookatRotation (Math|Vector|MakeVector 0.0 0.0 0.0) (.impactnormal Hit)) "TraceTypeQuery1" false 0 "Persistent"))
  (return (not (or _returnvalue_10 _returnvalue_11)) _returnvalue_8 _returnvalue_9))